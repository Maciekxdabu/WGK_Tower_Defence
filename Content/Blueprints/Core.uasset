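; Core Blueprint that holds the player's health, score and money, with getters for each.
; ReduceHealth subtracts damage and opens Menu_Level once health reaches zero or below, while IncreaseScore adds to the score.
; ChangeMoney applies a change only if the balance stays non-negative, but its returned Boolean repeats that check against the already updated balance.
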(event `ReduceHealth`
  (params (ReducedHealth :type Integer))
  (bind _output_get (set `self.Health` (- (`self.Health`) ReducedHealth)))
  (if (<= _output_get 0)
    (`GameplayStatics.OpenLevelBySoftObjectPtr` "/Game/Levels/Menu_Level.Menu_Level")))

(event `IncreaseScore`
  (params (AddedScore :type Integer))
  (set `self.Score` (+ AddedScore (`self.Score`))))

(fn `ChangeMoney`
  (params (ChangedValue :type Integer))
  (returns (Success :type Boolean))
  (bind _returnvalue (+ (`self.Money`) ChangedValue))
  (bind _returnvalue_2 (>= _returnvalue 0))
  (if _returnvalue_2
    (set `self.Money` _returnvalue))
  (return _returnvalue_2))

(fn `GetHealth`
  (returns (Health :type Integer))
  (return (`self.Health`)))

(fn `GetMoney`
  (returns (Money :type Integer))
  (return (`self.Money`)))

(fn `GetScore`
  (returns (Score :type Integer))
  (return (`self.Score`)))

(fn `UserConstructionScript`)