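; Buildable turret that, once built, shoots at in-range enemies, favoring those nearest the Core.
; Tick scans all Enemy actors, tracking the in-range one closest to the Core as CurrentTarget.
; A DoOnce and delay throttle projectile spawning, triggered mid-scan, so a shot can precede the final target choice.
; An overlap counter maintains the IsOverlapping flag against other structures, and the construction script scales the range circle to Range.
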(event `self.ReceiveActorBeginOverlap`
  (params (OtherActor :type "Actor Object Reference"))
  ;[1 1 1] Check for overlapping with other Structures
  (`/Engine/EditorBlueprintResources/StandardMacros.IncrementInt` (`self.OverlappingCounter`)
    (:`  `
      (set `self.IsOverlapping` true))))

(event `self.ReceiveActorEndOverlap`
  (params (OtherActor :type "Actor Object Reference"))
  ;[1 1 1] Check for overlapping with other Structures
  (bind _result (`/Engine/EditorBlueprintResources/StandardMacros.DecrementInt` (`self.OverlappingCounter`))
    (:`  `
      (if (== _result 0)
        (set `self.IsOverlapping` false)))))

(event `self.ReceiveTick`
  (params (DeltaSeconds :type "Float (single-precision)"))
  ;[1 1 1] Find Enemies in range
  (if (`self.isBuilt`)
    (bind _outactors (`GameplayStatics.GetAllActorsOfClass` "/Game/Blueprints/Enemy.Enemy_C"))
    (set `self.TargetDistanceToCore` -1.0)
    (set `self.CurrentTarget` (`self.EmptyEnemy`))
    (if (!= (`KismetArrayLibrary.Array_Length` _outactors) 0)
      (for _array_element _outactors
        (if (== (`self.TargetDistanceToCore`) -1.0)
          (bind _returnvalue (`SceneComponent.K2_GetComponentLocation` (`/Game/Blueprints/Enemy.DefaultSceneRoot` _array_element)))
          (bind _returnvalue_2 (> (- (`self.Range`) (`KismetMathLibrary.Vector_Distance` (`SceneComponent.K2_GetComponentLocation` (`self.TurretMesh`)) _returnvalue)) 0.0))
          (if _returnvalue_2
            (bind _returnvalue_3 (`KismetMathLibrary.Vector_Distance` _returnvalue (`SceneComponent.K2_GetComponentLocation` (`/Game/Blueprints/Core.DefaultSceneRoot` (stale `self.ReceiveBeginPlay` _returnvalue)))))
            (set `self.TargetDistanceToCore` _returnvalue_3 :!label _label)
            (bind _output_get (set `self.CurrentTarget` _array_element))
            (if (`KismetSystemLibrary.IsValid` _output_get)
              (`/Engine/EditorBlueprintResources/StandardMacros.DoOnce` false :!label _label_2
                (:`Completed`
                  (`self.FireAtTarget`)
                  (`KismetSystemLibrary.Delay` (`self.FireDelay`))
                  (goto _label_2 :!via `Reset`)))))
          (elif (and _returnvalue_2 (< _returnvalue_3 (`self.TargetDistanceToCore`)))
            (goto _label)))))))

(event `self.ReceiveBeginPlay`
  ;[1 1 1] Find Enemies in range
  (bind _returnvalue (`GameplayStatics.GetActorOfClass` "/Game/Blueprints/Core.Core_C")))

(fn `FireAtTarget`
  (bind _currenttarget (`self.CurrentTarget`))
  (bind _returnvalue (`SceneComponent.K2_GetComponentLocation` (`self.FiringArrow`)))
  (if (`KismetSystemLibrary.IsValid` _currenttarget)
    (`|SpawnActorFromClass` "/Game/Blueprints/Turrets/Projectile_BP.Projectile_BP_C" (`KismetMathLibrary.MakeTransform` _returnvalue (`KismetMathLibrary.FindLookAtRotation` _returnvalue (`self.K2_GetActorLocation` _currenttarget))) "AlwaysSpawn" "MultiplyWithRoot" null null)))

(fn `UserConstructionScript`
  (`SceneComponent.SetWorldScale3D` (`self.RangeCircle`) (`KismetMathLibrary.Conv_DoubleToVector` (/ (`self.Range`) 270.0))))