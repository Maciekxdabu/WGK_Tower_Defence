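; Enemy actor that travels along a spline path and destroys itself when it reaches the end.
; Each tick it accumulates time lived, multiplies it by Speed to get a distance, and moves its root to that world location on the spline without sweeping.
; Once that distance exceeds the spline length, it prints a debug message and destroys itself.
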(event `self.ReceiveTick`
  (params (DeltaSeconds :type "Float (single-precision)"))
  (bind _output_get (set `self.timeLived` (+ DeltaSeconds (`self.timeLived`))))
  (bind _returnvalue (* _output_get (`self.speed`)))
  (`SceneComponent.K2_SetWorldLocation` (`self.DefaultSceneRoot`) (`SplineComponent.GetLocationAtDistanceAlongSpline` (`self.spline`) _returnvalue "World") false false)
  (if (> _returnvalue (`SplineComponent.GetSplineLength` (`self.spline`)))
    (`KismetSystemLibrary.PrintString` "Enemy has reached the end! Initiating self-destruction!")
    (`self.K2_DestroyActor`)))

(fn `UserConstructionScript`
  (set `self.timeLived` 0.0))