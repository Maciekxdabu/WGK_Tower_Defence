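; Enemy spawner that releases enemy waves from level data onto a spline path, started with the N key.
; Each wave start queues up to three enemy types with amount and delay.
; Tick counts down each entry's delay independently, spawns actors at the spline transform with spline and core references, and removes exhausted entries mid-loop.
; A wave ends once everything has spawned, regardless of surviving enemies.
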(event `Key|N`
  (params (Key :type "Key Structure"))
  (:`Released`
    (if (not (`self.WaveOngoing`))
      (`self.StartNextWave`))))

(event `StartNextWave`
  (bind _result (`/Engine/EditorBlueprintResources/StandardMacros.IncrementInt` (`self.CurrentWave`))
    (:`  `
      (`KismetArrayLibrary.Array_Clear` (`self.EnemiesOnCurrentWave`))
      (bind (_enemy_1 _enemy_2 _enemy_3) (break `/Game/Blueprints/WaveData` (`|GetArrayItem` (`/Game/Blueprints/LevelData.Waves` (`self.LevelData`)) _result)))
      (for (_array_element _array_index) (`|MakeArray` _enemy_1 _enemy_2 _enemy_3)
        (bind (_delay _amount) (break `/Game/Blueprints/WaveEnemyData` _array_element))
        (if (> _amount 0)
          (`KismetArrayLibrary.Array_Add` (`self.EnemiesOnCurrentWave`) (make `/Game/Blueprints/WaveEnemy` (`|GetArrayItem` (`/Game/Blueprints/LevelData.EnemiesDic` (`self.LevelData`)) _array_index) _amount _delay _delay))))
      (set `self.WaveOngoing` true))))

(event `SpawnEnemy`
  (params (EnemyToSpawn :type "/Game/Blueprints/Enemy Class Reference"))
  (`|SpawnActorFromClass` EnemyToSpawn (`SplineComponent.GetTransformAtTime` (`self.Spline`) 0.0 "World" false false) "Undefined" "MultiplyWithRoot" null (`self.Spline`) (`self.CoreRef`) null))

(event `self.ReceiveTick`
  (params (DeltaSeconds :type "Float (single-precision)"))
  (bind _enemiesoncurrentwave (`self.EnemiesOnCurrentWave`))
  (if (`self.WaveOngoing`)
    (for (_array_element _array_index) _enemiesoncurrentwave
      (bind (_enemy _amount _delay _currentdelay) (break `/Game/Blueprints/WaveEnemy` _array_element))
      (bind _returnvalue (- _currentdelay DeltaSeconds))
      (if (<= _returnvalue 0.0)
        (`self.SpawnEnemy` _enemy)
        (bind _result (`/Engine/EditorBlueprintResources/StandardMacros.DecrementInt` _amount)
          (:`  `
            (if (<= _result 0)
              (`KismetArrayLibrary.Array_RemoveItem` (`self.EnemiesOnCurrentWave`) _array_element)
              (else
                (bind _structout (setmembers `/Game/Blueprints/WaveEnemy` :`StructRef` _array_element :`Amount` _result :`CurrentDelay` _delay))
                (`KismetArrayLibrary.Array_Set` (`self.EnemiesOnCurrentWave`) _array_index _structout)))))
        (else
          (bind _structout_2 (setmembers `/Game/Blueprints/WaveEnemy` :`StructRef` _array_element :`CurrentDelay` _returnvalue))
          (`KismetArrayLibrary.Array_Set` (`self.EnemiesOnCurrentWave`) _array_index _structout_2))))
    (if (`KismetArrayLibrary.Array_IsEmpty` _enemiesoncurrentwave)
      (set `self.WaveOngoing` false))))

(fn `UserConstructionScript`)