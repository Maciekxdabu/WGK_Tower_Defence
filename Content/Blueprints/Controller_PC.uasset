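; Player controller that runs mouse-driven placement for two selectable turret types.
; Select inputs toggle build mode or swap the preview turret; selecting the active type again destroys it and exits.
; Tick moves the preview to the cursor's deprojected ray intersection with the Z=0 plane, tinting it red when overlapping, green otherwise.
; A click on a clear spot leaves the turret untinted and spawns another preview for continued building.
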(event `self.ReceiveTick`
  (params (DeltaSeconds :type "Float (single-precision)"))
  (bind _is_building (`self.Is Building`))
  (bind _turretmesh (`/Game/Blueprints/BuildBase_BP.TurretMesh` (`self.Turret Being Built`)))
  (if _is_building
    (`self.Position Build Turret`)
    (if (and _is_building (stale `InputAction|Place Turret` _output_get) (not (`/Game/Blueprints/BuildBase_BP.IsOverlapping` (`self.Turret Being Built`))))
      (set `self.Click To Place` false)
      (`PrimitiveComponent.SetCollisionEnabled` _turretmesh "QueryOnly")
      (`MeshComponent.SetVectorParameterValueOnMaterials` _turretmesh "Tint" (1.0 1.0 1.0))
      (`self.Spawn Turret`)
      (else
        (set `self.Click To Place` false)))))

(event `InputAction|Place Turret`
  (params (Key :type "Key Structure"))
  (:`Pressed`
    (bind _output_get (set `self.Click To Place` true))))

(event `InputAction|Select Turret 1`
  (params (Key :type "Key Structure"))
  (:`Pressed`
    (set `self.Build Class` "/Game/Blueprints/BuildTurret1_BP.BuildTurret1_BP_C")
    (`self.Toggle Build Turret` :!label _label)))

(event `InputAction|Select Turret 2`
  (params (Key :type "Key Structure"))
  (:`Pressed`
    (set `self.Build Class` "/Game/Blueprints/BuildTurret2_BP.BuildTurret2_BP_C")
    (goto _label)))

(fn `Calculate Location`
  (returns (ReturnValue :type "Vector Structure"))
  (bind (_worldlocation _worlddirection) (`self.DeprojectMousePositionToWorld`))
  (return (+ _worldlocation (* (* _worlddirection (/ (.z _worldlocation) (.z _worlddirection))) (-1.0 -1.0 -1.0)))))

(fn `Position Build Turret`
  (bind _turret_being_built (`self.Turret Being Built`))
  (bind _turretmesh (`/Game/Blueprints/BuildBase_BP.TurretMesh` _turret_being_built))
  (bind _returnvalue (`self.Calculate Location`))
  (`self.K2_SetActorLocation` (`self.Turret Being Built`) _returnvalue false false)
  (if (`/Game/Blueprints/BuildBase_BP.IsOverlapping` _turret_being_built)
    (`MeshComponent.SetVectorParameterValueOnMaterials` _turretmesh "Tint" (0.4 0.0 0.02))
    (else
      (`MeshComponent.SetVectorParameterValueOnMaterials` _turretmesh "Tint" (0.0 0.3 0.03)))))

(fn `Spawn Turret`
  (bind _output_get (set `self.Previous Build Class` (`self.Build Class`)))
  (bind _returnvalue (`self.Calculate Location`))
  (bind _returnvalue_2 (`|SpawnActorFromClass` _output_get (`KismetMathLibrary.MakeTransform` _returnvalue) "AlwaysSpawn" "MultiplyWithRoot" null null))
  (bind _output_get_2 (set `self.Turret Being Built` _returnvalue_2))
  (bind _turretmesh (`/Game/Blueprints/BuildBase_BP.TurretMesh` _output_get_2))
  (`PrimitiveComponent.SetCollisionEnabled` _turretmesh "QueryOnly")
  (`MeshComponent.SetVectorParameterValueOnMaterials` _turretmesh "Tint" (0.0 0.3 0.03)))

(fn `Toggle Build Turret`
  (bind _turret_being_built (`self.Turret Being Built`))
  ;[1 1 1] Sprawdza, czy wyjsc z budowania, czy przelaczyc turret
  (if (`self.Is Building`)
    (if (== (`self.Build Class`) (`self.Previous Build Class`))
      (set `self.Is Building` false)
      (`self.K2_DestroyActor` _turret_being_built)
      (else
        (`self.K2_DestroyActor` _turret_being_built)
        (`self.Spawn Turret` :!label _label)))
    (else
      (set `self.Is Building` true)
      (set `self.Click To Place` false)
      (goto _label))))

(fn `UserConstructionScript`)