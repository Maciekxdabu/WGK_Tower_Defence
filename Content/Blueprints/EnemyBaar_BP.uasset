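; EnemyBaar_BP is a follower actor that tracks a referenced enemy, likely as its overhead bar.
; Each tick it sets its root's world transform to the enemy's location plus an offset, using a stored rotation instead of the enemy's own.
; It destroys itself once the enemy reference is no longer valid.
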(event `self.ReceiveTick`
  (params (DeltaSeconds :type "Float (single-precision)"))
  (bind _returnvalue_location (`KismetMathLibrary.BreakTransform` (`self.GetTransform` (`self.EnemyRef`))))
  (if (`KismetSystemLibrary.IsValid` (`self.EnemyRef`))
    (`SceneComponent.K2_SetWorldTransform` (`self.DefaultSceneRoot`) (`KismetMathLibrary.MakeTransform` (+ _returnvalue_location (`self.Offset`)) (`self.rotationVec`)) false false)
    (else
      (`self.K2_DestroyActor`))))

(fn `UserConstructionScript`)